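; Game mode blueprint that runs the level's audio and switches it when the quest HUD reports the end.
; BeginPlay caches the player's BP_QuestHUD and spawns an audio component, stored as Sound.
; Tick polls the HUD's IsEnd flag, stops Sound while it is set, and uses a DoOnce to spawn a second audio component a single time.
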(event EventBeginPlay
  (CallFunction|CastHUD)
  (bind _returnvalue (AddComponent|AddAudioComponent false))
  (Variables|Default|SetSound _returnvalue))

(event EventTick
  (params (DeltaSeconds :type Float%20%28single-precision%29))
  (bind _bp_quest_hud (Variables|Default|GetBP%20Quest%20HUD)
    (:then
      (if (Variables|/Script/QuestMapPrototype.QuestHUD|GetIsEnd _bp_quest_hud)
        (Audio|Components|Audio|Stop (Variables|Default|GetSound))
        (Utilities|FlowControl|DoOnce false
          (:Completed
            (AddComponent|AddAudioComponent false)))))
    (:else)))

(fn ConstructionScript)

(fn CastHUD
  (bind _asbp_quest_hud (Utilities|Casting|CastToBP_QuestHUD (HUD|GetHUD (Game|GetPlayerController 0))))
  (Variables|Default|SetBP%20Quest%20HUD _asbp_quest_hud))